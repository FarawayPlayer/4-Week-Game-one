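; Enemy Blueprint that is set up to move along the spline of a PatrolPath actor found in the level at BeginPlay.
; The EnemyMovement timeline lerps distance over the spline length to set world location, while rotation always samples the spline start in local space.
; The timeline's play rate is set to zero before playing, and the rate calculation from CompletionTime is left unconnected, so movement does not advance.
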(event Custom|MoveObject
  (bind _splineref (Variables|Default|GetSplineREF))
  (bind _spline (Variables|/Game/Ricardo/Enemy/PatrolPath-.PatrolPath-_C|GetSpline _splineref))
  (Components|Timeline|SetPlayRate (Variables|Default|GetEnemyMovement) 0.0)
  (bind _movement (Timeline|EnemyMovement Play)
    (:Update
      (Transformation|SetActorTransform (Math|Transform|MakeTransform (Spline|GetLocationatDistanceAlongSpline _spline (Math|Float|Lerp 0.0 (Spline|GetSplineLength (Variables|/Game/Ricardo/Enemy/PatrolPath-.PatrolPath-_C|GetSpline (Variables|Default|GetSplineREF))) _movement) "World") (Spline|GetRotationatDistanceAlongSpline _spline 0.0 "Local") "1.000000,1.000000,1.000000")))))

(event EventBeginPlay
  (bind _returnvalue (Actor|GetActorOfClass "/Game/Ricardo/Enemy/PatrolPath-.PatrolPath-_C"))
  (Variables|Default|SetSplineREF _returnvalue)
  (CallFunction|MoveObject))

(fn ConstructionScript)