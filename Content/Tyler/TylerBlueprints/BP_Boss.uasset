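; 2D flipbook boss that fires a timed laser, hurting the player or showing the death screen if health is depleted.
; Player overlaps with DamageZone reduce boss health and knock the player sideways; zero health plays death effects, pauses and shows the finish widget.
; While Active, Tick impulses move it between two Bp_BossMovePoint actors, then toward a third after 12 seconds, while CheckHight corrects Y/Z drift.
; StartAttack and Active are not triggered within this graph.
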(event OnComponentBeginOverlap(DamageZone)
  (params (OverlappedComponent :type Primitive%20Component%20Object%20Reference) (OtherActor :type Actor%20Object%20Reference) (OtherComp :type Primitive%20Component%20Object%20Reference) (OtherBodyIndex :type Integer) (bFromSweep :type Boolean) (SweepResult :type Hit%20Result%20Structure%20%28by%20ref%29))
  (bind _ref_to_player (Variables|Default|Getref%20to%20player))
  (bind _charactermovement (Variables|/Script/Engine.Character|GetCharacterMovement _ref_to_player))
  ;[1 1 1] Boss takes damage
  (Utilities|Casting|CastToBP_PlayerCharacter OtherActor)
  (Variables|Default|SetCurrentHealth (- (Variables|Default|GetCurrentHealth) 25.0))
  (CallFunction|UpdateHealthBoss)
  (Audio|PlaySound2D "/Game/Ricardo/Sounds/8-bit-cannon-fire-96505.8-bit-cannon-fire-96505" 1.0 1.0 0.0 0 0)
  (if (> (.x (Transformation|GetWorldLocation (Variables|Collision|GetCapsuleComponent))) (.x (Transformation|GetWorldLocation (Variables|/Script/Paper2D.PaperCharacter|GetSprite _ref_to_player))))
    (Physics|AddImpulse _charactermovement "-500.000000,0.000000,0.000000" true)
    (else
      (Physics|AddImpulse _charactermovement "500.000000,0.000000,0.000000" true))))

(event OnComponentBeginOverlap(LaserDamage)
  (params (OverlappedComponent :type Primitive%20Component%20Object%20Reference) (OtherActor :type Actor%20Object%20Reference) (OtherComp :type Primitive%20Component%20Object%20Reference) (OtherBodyIndex :type Integer) (bFromSweep :type Boolean) (SweepResult :type Hit%20Result%20Structure%20%28by%20ref%29))
  ;[1 1 1] Damage from laser
  (bind _asbp_player_character (Utilities|Casting|CastToBP_PlayerCharacter OtherActor))
  (Utilities|FlowControl|DoOnce false :!label _label
    (:Completed
      (Utilities|FlowControl|Sequence
        (:then_0
          (if (Variables|/Script/Engine.SceneComponent|GetbVisible (Variables|Default|GetLaser))
            (if (<= (Variables|/Game/Tyler/TylerBlueprints/BP_PlayerCharacter.BP_PlayerCharacter_C|GetHealth _asbp_player_character) 0.0)
              (bind _returnvalue (UserInterface|CreateWidget "/Game/Ricardo/Health/Death_Widget.Death_Widget_C"))
              (UserInterface|Viewport|AddtoViewport _returnvalue 0)
              (Audio|PlaySound2D "/Game/Ricardo/Sounds/8-bit-video-game-fail-version-2-145478.8-bit-video-game-fail-version-2-145478" 1.0 1.0 0.0 0 0)
              (Game|SetGamePaused true)
              (Variables|/Script/Engine.PlayerController|SetbShowMouseCursor (Game|GetPlayerController (Variables|/Script/Engine.Pawn|GetPlayerState (Game|GetPlayerCharacter 0))) true)
              (else
                (Default|RemoveHealthBoss _asbp_player_character)))))
        (:then_1
          (Utilities|FlowControl|Delay 2.0)
          (goto _label Reset))))))

(event Custom|StartAttack
  ;[1 1 1] Attack animation and damage
  (Sprite|SetFlipbook (Variables|Default|GetSprite) "/Game/Tyler/Assests/BossAttack1.BossAttack1")
  (Utilities|FlowControl|Delay 1.0)
  (Rendering|SetVisibility (Variables|Default|GetLaser) true false)
  (Sprite|SetFlipbook (Variables|Default|GetSprite) "/Game/Tyler/Assests/BossAttackHold.BossAttackHold")
  (Sprite|SetFlipbook (Variables|Default|GetLaser) "/Game/Tyler/Assests/LaserHold.LaserHold")
  (Collision|SetCollisionEnabled (Variables|Default|GetLaserDamage) "QueryOnly")
  (bind _returnvalue (Audio|SpawnSound2D "/Game/Ricardo/Sounds/8-bit-laser-151672.8-bit-laser-151672" 1.0 1.0 0.0 0 false false))
  (Utilities|FlowControl|Delay 5.0)
  (Rendering|SetVisibility (Variables|Default|GetLaser) false false)
  (Collision|SetCollisionEnabled (Variables|Default|GetLaserDamage) "NoCollision")
  (Sprite|SetFlipbook (Variables|Default|GetSprite) "/Game/Tyler/Assests/BossIdle1.BossIdle1")
  (Sprite|SetFlipbook (Variables|Default|GetLaser) "/Game/Tyler/Assests/laser3.laser3")
  (Components|Activation|SetActive _returnvalue false false))

(event Custom|Update%20health%20boss
  ;[1 1 1] Update boss health
  (Variables|Default|SetPercentHealth (/ (Variables|Default|GetCurrentHealth) (Variables|Default|GetTotalHealth)))
  (if (<= (Variables|Default|GetCurrentHealth) 0.0) ; Boss is dead
    (bind _returnvalue (Audio|SpawnSound2D "/Game/Ricardo/Sounds/crash04-84461.crash04-84461" 1.0 1.0 0.0 0))
    (Sprite|SetFlipbook (Variables|Default|GetSprite) "/Game/Tyler/SunnyLandAssests/sprites/enemy-death/enemy-death.enemy-death")
    (Utilities|FlowControl|Delay 1.0)
    (Components|Activation|SetActive _returnvalue false false)
    (Game|SetGamePaused true)
    (Audio|PlaySound2D "/Game/Ricardo/Sounds/win-sfx-38507.win-sfx-38507" 1.0 1.0 0.0 0 0)
    (bind _returnvalue_2 (UserInterface|CreateWidget "/Game/Ricardo/GameEnds/FinishGame_Widget.FinishGame_Widget_C"))
    (UserInterface|Viewport|AddtoViewport _returnvalue_2 0)
    (Audio|PlaySound2D "/Game/Ricardo/Sounds/playing-in-the-forest-152450.playing-in-the-forest-152450" 1.0 1.0 0.0 0 0)))

(event Custom|MovePoints
  (bind _capsulecomponent (Variables|Collision|GetCapsuleComponent))
  (bind _returnvalue (Transformation|GetWorldLocation _capsulecomponent))
  ;[1 1 1] Boss movement
  ;;[1 1 1] Two points code
  (if (Variables|Default|GetMovePoint)
    (if (> (.x _returnvalue) (.x (Transformation|GetWorldLocation (Variables|/Script/Engine.Actor|GetRootComponent (Utilities|Array|Get(acopy) (stale EventBeginPlay _outactors_2))))))
      (Physics|AddImpulse (Variables|Character|GetCharacterMovement) "-2.000000,0.000000,0.000000" true)
      (else
        (Variables|Default|SetMovePoint false)))
    (elif (> (.x _returnvalue) (.x (Transformation|GetWorldLocation (Variables|/Script/Engine.Actor|GetRootComponent (Utilities|Array|Get(acopy) (stale EventBeginPlay _outactors_2) 1)))))
      (Variables|Default|SetMovePoint true)
      (else
        (Physics|AddImpulse (Variables|Character|GetCharacterMovement) "2.000000,0.000000,0.000000" true)))))

(event Custom|CheckHight
  (bind _capsulecomponent (Variables|Collision|GetCapsuleComponent))
  (bind _returnvalue (Transformation|GetWorldLocation _capsulecomponent))
  ;[1 1 1] Checks if hight has change, if so then fix it
  (Utilities|FlowControl|Sequence
    (:then_0
      (if (not (== (.y _returnvalue) 0.0)) ; fix y not 0
        (Transformation|SetWorldTransform (Variables|Collision|GetCapsuleComponent) (Math|Transform|MakeTransform (Math|Vector|MakeVector (.x _returnvalue) 0.0 -91.0) "0, 0, 0" "1.000000,1.000000,1.000000") false false)))
    (:then_1
      (if (not (== (.z _returnvalue) -91.0)) ; fix z not -91
        (Transformation|SetWorldTransform (Variables|Collision|GetCapsuleComponent) (Math|Transform|MakeTransform (Math|Vector|MakeVector (.x _returnvalue) (.y _returnvalue) -91.0) "0, 0, 0" "1.000000,1.000000,1.000000") false false)))))

(event EventBeginPlay
  ;[1 1 1] Ref to player and points
  (bind _outactors (Actor|GetAllActorsOfClass "/Game/Tyler/TylerBlueprints/BP_PlayerCharacter.BP_PlayerCharacter_C"))
  (Variables|Default|Setref%20to%20player (Utilities|Array|Get(acopy) _outactors))
  (bind _outactors_2 (Actor|GetAllActorsOfClass "/Game/Tyler/TylerBlueprints/Bp_BossMovePoint.Bp_BossMovePoint_C")))

(event Collision|EventActorBeginOverlap
  (params (OtherActor :type Actor%20Object%20Reference)))

(event EventTick
  (params (DeltaSeconds :type Float%20%28single-precision%29))
  ;[1 1 1] Boss movement
  ;;[1 1 1] Boss moves back and forth from two points down to one ppoint
  (CallFunction|CheckHight)
  (if (Variables|Default|GetActive)
    (if (Variables|Default|GetOnePoint)
      (CallFunction|MovePoints)
      (Utilities|FlowControl|DoOnce false
        (:Completed
          (Utilities|FlowControl|Delay 12.0)
          (Variables|Default|SetOnePoint false)))
      (elif (> (.x (Transformation|GetWorldLocation (Variables|Collision|GetCapsuleComponent))) (.x (Transformation|GetWorldLocation (Variables|/Game/Tyler/TylerBlueprints/Bp_BossMovePoint.Bp_BossMovePoint_C|GetDefaultSceneRoot (Utilities|Array|Get(acopy) (stale EventBeginPlay _outactors_2) 2)))))
        (Physics|AddImpulse (Variables|Character|GetCharacterMovement) "-2.000000,0.000000,0.000000" true)
        (else
          (Physics|AddImpulse (Variables|Character|GetCharacterMovement) "2.000000,0.000000,0.000000" true))))))

(fn ConstructionScript)