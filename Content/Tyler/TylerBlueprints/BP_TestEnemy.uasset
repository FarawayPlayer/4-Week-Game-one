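; Test 2D side-scroller enemy that chases the player and can be killed by jumping on it.
; While alive and the player is inside the Tracking overlap, Tick applies horizontal velocity impulses toward the player and flips the sprite.
; A capsule hit from a falling player disables collision, plays the death flipbook, then destroys the enemy.
; Other hits remove player health, throttled by a DoOnce with delayed reset.
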(event OnComponentBeginOverlap(Tracking)
  (params (OverlappedComponent :type Primitive%20Component%20Object%20Reference) (OtherActor :type Actor%20Object%20Reference) (OtherComp :type Primitive%20Component%20Object%20Reference) (OtherBodyIndex :type Integer) (bFromSweep :type Boolean) (SweepResult :type Hit%20Result%20Structure%20%28by%20ref%29))
  (Utilities|Casting|CastToBP_PlayerCharacter OtherActor)
  (Variables|Default|SetPlayerInRange true))

(event OnComponentHit(CapsuleComponent)
  (params (HitComponent :type Primitive%20Component%20Object%20Reference) (OtherActor :type Actor%20Object%20Reference) (OtherComp :type Primitive%20Component%20Object%20Reference) (NormalImpulse :type Vector :default "0, 0, 0") (Hit :type Hit%20Result%20Structure%20%28by%20ref%29))
  ;[1 1 1] Enemy Damage and Deaths
  (bind _asbp_player_character (Utilities|Casting|CastToBP_PlayerCharacter OtherActor)) ; Hit player
  (if (AI|Components|NavMovement|IsFalling (Variables|/Script/Engine.Character|GetCharacterMovement _asbp_player_character)) ; if player is falling then kill enemy
    (Collision|SetCollisionEnabled (Variables|Collision|GetCapsuleComponent) "NoCollision") ; remove collision
    (Variables|Default|SetIsDead true) ; this is to stop walking
    (Sprite|SetFlipbook (Variables|Default|GetSprite) "/Game/Tyler/SunnyLandAssests/sprites/enemy-death/enemy-death.enemy-death") ; change to death animation
    (Utilities|FlowControl|Delay 0.5) ; delay so death animation plays
    (Actor|DestroyActor)
    (else
      ;[1 1 1] Player takes damage
      (Utilities|FlowControl|DoOnce false :!label _label
        (:Completed
          (Default|RemoveHealth (Variables|Default|GetReftoPlayer))
          (Utilities|FlowControl|Delay 1.0)
          (goto _label Reset))))))

(event OnComponentEndOverlap(Tracking)
  (params (OverlappedComponent :type Primitive%20Component%20Object%20Reference) (OtherActor :type Actor%20Object%20Reference) (OtherComp :type Primitive%20Component%20Object%20Reference) (OtherBodyIndex :type Integer))
  (Utilities|Casting|CastToBP_PlayerCharacter OtherActor)
  (Variables|Default|SetPlayerInRange false))

(event Collision|EventActorBeginOverlap
  (params (OtherActor :type Actor%20Object%20Reference)))

(event EventTick
  (params (DeltaSeconds :type Float%20%28single-precision%29))
  ;[1 1 1] Enemy Movment
  (if (and (Math|Boolean|NORBoolean (Variables|Default|GetIsDead) false) (Variables|Default|GetPlayerInRange)) ; Check is enemy is dead
    (if (> (.x (Transformation|GetWorldLocation (Variables|Collision|GetCapsuleComponent))) (.x (Transformation|GetWorldLocation (Variables|/Script/Paper2D.PaperCharacter|GetSprite (Variables|Default|GetReftoPlayer)))))
      (Physics|AddImpulse (Variables|Character|GetCharacterMovement) "-70.000000,0.000000,0.000000" true) ; If player is on left
      (Transformation|SetWorldRotation (Variables|Default|GetSprite) "0.000000,180.000000,0.000000" false false)
      (else
        (Physics|AddImpulse (Variables|Character|GetCharacterMovement) "70.000000,0.000000,0.000000" true) ; if player is on right
        (Transformation|SetWorldRotation (Variables|Default|GetSprite) "0, 0, 0" false false)))))

(event EventBeginPlay
  ;[1 1 1] ref to player character
  (bind _outactors (Actor|GetAllActorsOfClass "/Game/Tyler/TylerBlueprints/BP_PlayerCharacter.BP_PlayerCharacter_C"))
  (Variables|Default|SetReftoPlayer (Utilities|Array|Get(acopy) _outactors)))

(fn ConstructionScript)